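; SnowmanPawn_BP is a player-input pawn that slides along the world X or Y axis.
; MoveX and MoveY axis events store clamped values and flag which axis is active.
; Tick scales that value by delta time and a speed multiplier, then sets location without sweep, with X taking priority, so no diagonal movement.
; It reads its position through GetActorOfClass on its own class rather than self.
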(event EventBeginPlay)

(event Collision|EventActorBeginOverlap
  (params (OtherActor :type Actor%20Object%20Reference)))

(event EventTick
  (params (DeltaSeconds :type Float%20%28single-precision%29))
  (if (Variables|Default|GetalongX)
    (bind _returnvalue (Actor|GetActorOfClass "SnowmanPawn_BP_C"))
    (bind _output_get (Variables|Default|SetLocation%20X (.X (Math|Vector|BreakVector (Transformation|GetActorLocation _returnvalue)))))
    (bind _output_get_2 (Variables|Default|SetLocation%20X (+ _output_get (* (Variables|Default|GetmovementX) DeltaSeconds (Variables|Default|GetSPEED%20MULTIPLIER)))))
    (Transformation|SetActorLocation (Math|Vector|MakeVector _output_get_2 (.Y (Math|Vector|BreakVector (Transformation|GetActorLocation _returnvalue))) (.Z (Math|Vector|BreakVector (Transformation|GetActorLocation _returnvalue)))) false false)
    (elif (Variables|Default|GetalongY)
      (bind _returnvalue_2 (Actor|GetActorOfClass "SnowmanPawn_BP_C"))
      (bind _output_get_3 (Variables|Default|SetLocation%20Y (.Y (Math|Vector|BreakVector (Transformation|GetActorLocation _returnvalue_2)))))
      (bind _output_get_4 (Variables|Default|SetLocation%20Y (+ _output_get_3 (* (Variables|Default|GetmovementY) DeltaSeconds (Variables|Default|GetSPEED%20MULTIPLIER)))))
      (Transformation|SetActorLocation (Math|Vector|MakeVector (.X (Math|Vector|BreakVector (Transformation|GetActorLocation _returnvalue_2))) _output_get_4 (.Z (Math|Vector|BreakVector (Transformation|GetActorLocation _returnvalue_2)))) false false))))

(event Input|AxisEvents|InputAxisMoveX
  (params (AxisValue :type Float%20%28single-precision%29))
  (bind _output_get (Variables|Default|SetmovementX (Math|Float|Clamp(Float) AxisValue -1.0)))
  (Variables|Default|SetalongX (!= _output_get 0.0)))

(event Input|AxisEvents|InputAxisMoveY
  (params (AxisValue :type Float%20%28single-precision%29))
  (bind _output_get (Variables|Default|SetmovementY (Math|Float|Clamp(Float) AxisValue -1.0)))
  (Variables|Default|SetalongY (!= _output_get 0.0)))

(fn ConstructionScript)